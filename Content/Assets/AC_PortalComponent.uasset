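; Portal component that places a linked pair of portals (A and B) on portal walls.
; SpawnVectorAlongVector line-traces along a direction, asks the hit BP_PortalWall for a placement position, and spawns a wall-aligned BP_Portal there.
; SwapPortals destroys the previous portal in the chosen slot and stores the new one by reference, then both portals are re-linked.
; Spawned portals are tracked in PortalsOnWall and removed through their OnDestroyed event.
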(event EventBeginPlay)

(event EventTick
  (params (DeltaSeconds :type Float%20%28single-precision%29)))

(fn SpawnVectorAlongVector
  (params (StartLocation :type Vector) (Direction :type Vector) (PortalA :type Boolean))
  (bind (_outhit _returnvalue) (Collision|LineTraceForObjects StartLocation (+ StartLocation (* Direction (Variables|Constants|GetMaxSpawnDistance))) (Utilities|Array|MakeArray "ObjectTypeQuery8") false 0 "ForDuration"))
  (if _returnvalue
    (bind _asbp_portal_wall (Utilities|Casting|CastToBP_PortalWall (.HitActor (Collision|BreakHitResult _outhit))))
    (bind _returnvalue_2 (Class|APortalWall|CalculatePortalPosition _asbp_portal_wall (+ (.Location (Collision|BreakHitResult _outhit)) (Math|Vector|Normalize (- (.TraceStart (Collision|BreakHitResult _outhit)) (.TraceEnd (Collision|BreakHitResult _outhit)))))))
    (bind _returnvalue_3 (Game|SpawnActorfromClass "/Game/Assets/BP_Portal.BP_Portal_C" (Math|Transform|MakeTransform (Math|Transform|TransformLocation (Transformation|GetActorTransform _asbp_portal_wall) _returnvalue_2) (Transformation|GetActorRotation _asbp_portal_wall) "1.000000,1.000000,1.000000") "AlwaysSpawn" "MultiplyWithRoot" 0 PortalA 0))
    (Utilities|Array|Add (Variables|Default|GetPortalsOnWall) _returnvalue_3)
    (Game|BindEventtoOnDestroyed _returnvalue_3 (EventDispatchers|CreateEvent :!event OnPortalDestroyed))
    (bind _output_get (LocalVariables|SetNewPortal _returnvalue_3))
    (Utilities|IsValid _output_get
      (:Is%20Valid
        (CallFunction|SwapPortals (select PortalA (Variables|Default|GetPortalA) (Variables|Default|GetPortalB)) _output_get)
        (Utilities|FlowControl|Sequence
          (:then_0
            (bind _portala (Variables|Default|GetPortalA)
              (:then
                (Default|LinkPörtal _portala (Variables|Default|GetPortalB)))
              (:else)))
          (:then_1
            (bind _portalb (Variables|Default|GetPortalB)
              (:then
                (Default|LinkPörtal _portalb (Variables|Default|GetPortalA)))
              (:else))))))))

(fn OnPortalDestroyed
  (params (DestroyedActor :type Actor%20Object%20Reference))
  (Utilities|Array|RemoveItem (Variables|Default|GetPortalsOnWall) DestroyedActor))

(fn SwapPortals
  (params (OldPortal :type BP%20Portal%20Object%20Reference%20%28by%20ref%29) (NewPortal :type BP%20Portal%20Object%20Reference))
  (Utilities|FlowControl|Sequence
    (:then_0
      (Utilities|IsValid OldPortal
        (:Is%20Valid
          (Actor|DestroyActor OldPortal))))
    (:then_1
      (|SetBy-RefVar OldPortal NewPortal))))